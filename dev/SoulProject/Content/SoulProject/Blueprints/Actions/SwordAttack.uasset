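; Sword attack action actor that attaches to its owner, swings a sword through an arc and damages enemies it touches.
; Tick converts elapsed time over the attack duration into an angle, rotating SwordFB around the Y axis at a set range.
; Overlaps apply damage on the server only, skipping self and owner and checking faction state.
; The action completes and destroys itself when the swing ends; the construction script previews the arc position in editor.
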(event `self.ReceiveBeginPlay`
  (`parent.ReceiveBeginPlay`)
  (`self.UpdateSwordTransform` 0.0) ; Init location
  (`self.K2_AttachToActor` (`self.GetOwner`) "None" "SnapToTarget" "SnapToTarget" "SnapToTarget"))

(event `self.ReceiveTick`
  (params (DeltaSeconds :type "Float (single-precision)"))
  (`parent.ReceiveTick` DeltaSeconds)
  (`self.UpdateSwordMotion` DeltaSeconds))

(event `OnSwordMotionCompleted`
  (`self.CompleteAction`)
  (`self.K2_DestroyActor`))

(event `self.SwordFB.OnComponentBeginOverlap`
  (params (OverlappedComponent :type "PrimitiveComponent Object Reference") (OtherActor :type "Actor Object Reference") (OtherComp :type "PrimitiveComponent Object Reference") (OtherBodyIndex :type Integer) (bFromSweep :type Boolean) (SweepResult :type "HitResult Structure (by ref)"))
  (`/Engine/EditorBlueprintResources/ActorMacros.Switch Has Authority`
    (:`Authority`
      (`self.IgnoreSelfAndOwner` OtherActor
        (:`  `
          (bind _factionstate (`/Game/SoulProject/Blueprints/Libraries/Factions/FactionLibrary.GetFactionStateOfActors` self OtherActor))
          (switch `/Game/SoulProject/Blueprints/Libraries/Factions/FactionState` _factionstate
            (:`NewEnumerator2`
              (`GameplayStatics.ApplyDamage` OtherActor (`KismetMathLibrary.Conv_IntToDouble` (`self.Damages`)) (`self.GetInstigatorController`) self "/Script/Engine.DamageType"))))))))

(fn `UpdateSwordMotion`
  (params (DeltaTime :type "Float (double-precision)"))
  (locals (Ratio :type "Float (double-precision)" :default 0.0))
  (bind _output_get (set `self.ElapsedTime` (+ DeltaTime (`self.ElapsedTime`))))
  (bind _output_get_2 (set `local.Ratio` (`KismetMathLibrary.FClamp` (/ _output_get (`self.AttackDuration`)))))
  (`self.UpdateSwordTransform` _output_get_2)
  (if (`KismetMathLibrary.NearlyEqual_FloatFloat` (`local.Ratio`) 1.0)
    (`self.OnSwordMotionCompleted`)))

(fn `UpdateSwordTransform`
  (params (RotationRatio :type "Float (double-precision)"))
  (locals (Angle :type "Float (double-precision)"))
  (bind _rotationstart (`self.RotationStart`))
  (set `local.Angle` (`KismetMathLibrary.Lerp` _rotationstart (+ _rotationstart (`self.RotationRange`)) RotationRatio))
  (`SceneComponent.K2_SetRelativeLocationAndRotation` (`self.SwordFB`) (`KismetMathLibrary.RotateAngleAxis` (`KismetMathLibrary.MakeVector` 0.0 0.0 (`self.SwordRange`)) (`local.Angle`) (0.0 1.0 0.0)) (`KismetMathLibrary.MakeRotator` 0.0 (`/Game/SoulProject/Blueprints/Libraries/MathLibrary.SwitchFloatSign` (`local.Angle`))) false false))

(fn `UserConstructionScript`
  (`parent.UserConstructionScript`)
  (`self.UpdateSwordTransform` (`self.Editor_RotationRatio`)))