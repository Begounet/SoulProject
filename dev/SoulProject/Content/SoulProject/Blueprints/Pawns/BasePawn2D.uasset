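; Base 2D pawn that provides health, damage handling and faction queries for the game's sprite-based pawns.
; Any damage is truncated and applied to the Life component, destroying the pawn on death or otherwise granting timed invincibility when a post-hit duration is set.
; The sprite is tinted while Life reports invincibility.
; Helpers read the faction from the controller and resolve whether another actor is an enemy through relative faction state.
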(event `self.ReceiveAnyDamage`
  (params (Damage :type "Float (single-precision)") (DamageType :type "DamageType Object Reference") (InstigatedBy :type "Controller Object Reference") (DamageCauser :type "Actor Object Reference"))
  (bind _life (`self.Life`))
  (`parent.ReceiveAnyDamage` Damage DamageType InstigatedBy DamageCauser)
  (`LifeComponent.ApplyDamages` _life (`KismetMathLibrary.FTrunc` Damage))
  (if (`LifeComponent.IsDead` _life)
    (`self.K2_DestroyActor`)
    (else
      (`self.ApplyAfterHitInvincibility`))))

(event `self.Life.OnInvincibilityModeChanged`
  (params (LifeComponent :type "LifeComponent Object Reference") (bIsInvincible :type Boolean))
  (`PaperFlipbookComponent.SetSpriteColor` (`self.Sprite`) (select `bool` bIsInvincible :`false` (struct :`R` 1.0 :`G` 1.0 :`B` 1.0 :`A` 1.0) :`true` (struct :`R` 0.73 :`G` 0.634961 :`B` 0.102944 :`A` 1.0) :!type "LinearColor Structure")))

(fn `ApplyAfterHitInvincibility`
  (bind _invincibilitydurationafterhit (`self.InvincibilityDurationAfterHit`))
  (if (and (> _invincibilitydurationafterhit 0.0) (not (`LifeComponent.IsInvincible` (`self.Life`))))
    (`LifeComponent.EnableTimedInvincibility` (`self.Life`) _invincibilitydurationafterhit)))

(fn `GetFaction`
  (returns (Faction :type "/Game/SoulProject/Blueprints/Libraries/Factions/Faction Enum"))
  (bind _faction (`/Game/SoulProject/Blueprints/Libraries/Factions/FactionLibrary.GetActorFaction` (`self.GetController`)))
  (return _faction))

(fn `GetRelativeFactionState`
  (params (Actor :type "Actor Object Reference"))
  (returns (FactionState :type "/Game/SoulProject/Blueprints/Libraries/Factions/FactionState Enum"))
  (bind _factionstate (`/Game/SoulProject/Blueprints/Libraries/Factions/FactionLibrary.GetFactionStateOfActors` Actor self))
  (return _factionstate))

(fn `IsEnemy`
  (params (Actor :type "Actor Object Reference"))
  (returns (Enemy :type Boolean))
  (bind _factionstate (`self.GetRelativeFactionState` Actor))
  (return (select `/Game/SoulProject/Blueprints/Libraries/Factions/FactionState` _factionstate :`NewEnumerator2` true)))

(fn `UserConstructionScript`)