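; StandardPlayerCamera is a side-view camera that follows the player's controlled pawn.
; On becoming the view target it stores that pawn as Target, and it clears it when it stops being the view target.
; Each tick it matches the target's X and Z, uses DistanceFromTarget as an absolute world Y, and rotates to look at the target, with no smoothing.
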(event `self.ReceiveTick`
  (params (DeltaSeconds :type "Float (single-precision)"))
  (`parent.ReceiveTick` DeltaSeconds)
  (`self.UpdateCameraTransform` DeltaSeconds))

(event `self.K2_OnBecomeViewTarget`
  (params (PC :type "PlayerController Object Reference"))
  (set `self.Target` (`Controller.K2_GetPawn` PC)))

(event `self.K2_OnEndViewTarget`
  (params (PC :type "PlayerController Object Reference"))
  (set `self.Target` null))

(fn `UpdateCameraTransform`
  (params (DeltaSeconds :type "Float (double-precision)"))
  (locals (StartLocation :type "Vector Structure"))
  (bind _target (`self.Target`))
  (bind _returnvalue (`KismetMathLibrary.MakeVector` (.x (`self.K2_GetActorLocation` _target)) (`self.DistanceFromTarget`) (.z (`self.K2_GetActorLocation` _target))))
  (`/Engine/EditorBlueprintResources/StandardMacros.IsValid` _target
    (:`Is Valid`
      (set `local.StartLocation` _returnvalue)
      (`self.K2_SetActorLocationAndRotation` _returnvalue (`KismetMathLibrary.FindLookAtRotation` (`local.StartLocation`) (`self.K2_GetActorLocation` (`self.Target`)))))))

(fn `UserConstructionScript`)