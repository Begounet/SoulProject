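; BP_LifeComponent is a component that tracks an owner's integer life, with functions to apply damage, heal, check whether it is alive and get the life ratio.
; Damage and healing both route through SetLife, which clamps CurrentLife between zero and MaxLife.
; CurrentLife uses RepNotify, whose OnRep function broadcasts the OnLifeValueChanged dispatcher so listeners can react to changes.
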(fn `ApplyDamages`
  (params (Damages :type Integer))
  (`self.SetLife` (- (`self.CurrentLife`) Damages)))

(fn `GetLifeRatio`
  (returns (LifeRatio :type "Float (double-precision)"))
  (return (/ (`KismetMathLibrary.Conv_IntToDouble` (`self.CurrentLife`)) (`KismetMathLibrary.Conv_IntToDouble` (`self.MaxLife`)))))

(fn `Heal`
  (params (HealAmount :type Integer))
  (`self.SetLife` (+ HealAmount (`self.CurrentLife`))))

(fn `IsAlive`
  (returns (IsAlive :type Boolean))
  (return (> (`self.CurrentLife`) 0)))

(fn `OnRep_CurrentLife`
  (`self.OnLifeValueChanged`))

(fn `SetLife`
  (params (Life :type Integer))
  (set `self.CurrentLife` (`KismetMathLibrary.Clamp` Life 0 (`self.MaxLife`))))